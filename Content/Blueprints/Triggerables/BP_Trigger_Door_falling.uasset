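; Triggerable falling door that swings a wall out of the way by rotating it on its hinge.
; BeginPlay stores the hinge's world rotation and an end rotation offset in roll, then triggers immediately if IsPlayReady is false.
; Trigger plays a 2D sound and runs a timeline that lerps the hinge between the two rotations.
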(event `self.ReceiveBeginPlay`
  ;[1 1 1] Store the start rotations
  (bind _output_get (set `self.StartRotation` (`SceneComponent.K2_GetComponentRotation` (`self.Hinge`))))
  (set `self.EndRotation` (`KismetMathLibrary.MakeRotator` (+ (.roll _output_get) 100.0) (.pitch _output_get) (.yaw _output_get)))
  (if (not (`self.IsPlayReady`))
    (`/Game/Blueprints/Triggerables/BP_Triggerable.Trigger`)))

(event `/Game/Blueprints/Triggerables/BP_Triggerable.Trigger`
  ;[1 1 1] Animates and moves the wall out of the way
  (`GameplayStatics.PlaySound2D` null 1.0 1.0 0.0 null null)
  (bind (_direction _alpha) (`Timeline|Timeline` :`NewTime` (`self.PlayTime`))
    (:`Update`
      (`SceneComponent.K2_SetWorldRotation` (`self.Hinge`) (`KismetMathLibrary.RLerp` (`self.StartRotation`) (`self.EndRotation`) _alpha) false false))))

(fn `UserConstructionScript`
  (`parent.UserConstructionScript`))