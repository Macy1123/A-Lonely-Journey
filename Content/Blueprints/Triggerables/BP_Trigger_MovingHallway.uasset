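; BP_Trigger_MovingHallway is a triggerable moving hallway piece that slides its Cube to an offset position when triggered.
; At BeginPlay it caches the Cube's relative start location and builds the end location by adding IncreaseAmount along each entry in Directions.
; Trigger plays the MovementAlpha timeline, lerping the Cube between the two locations without sweep.
; The construction script applies the configurable Material to the Cube.
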(event `self.ReceiveBeginPlay`
  (bind (_endlocation_x _endlocation_y _endlocation_z) (`KismetMathLibrary.BreakVector` (`self.EndLocation`)))
  (bind (_endlocation_x_2 _endlocation_y_2 _endlocation_z_2) (`KismetMathLibrary.BreakVector` (`self.EndLocation`)))
  (bind (_endlocation_x_3 _endlocation_y_3 _endlocation_z_3) (`KismetMathLibrary.BreakVector` (`self.EndLocation`)))
  (bind (_endlocation_x_4 _endlocation_y_4 _endlocation_z_4) (`KismetMathLibrary.BreakVector` (`self.EndLocation`)))
  (bind (_endlocation_x_5 _endlocation_y_5 _endlocation_z_5) (`KismetMathLibrary.BreakVector` (`self.EndLocation`)))
  (bind (_endlocation_x_6 _endlocation_y_6 _endlocation_z_6) (`KismetMathLibrary.BreakVector` (`self.EndLocation`)))
  ;[1 1 1] Sets the start location
  (bind _output_get (set `self.StartLocation` (`SceneComponent.RelativeLocation` (`self.Cube`))))
  (set `self.EndLocation` _output_get)
  (for _array_element (`self.Directions`)
    ;[1 1 1] Depending on what direction the player sets and distance used, it wall add the neccisary amount to the end location that would be used later
    (switch `/Game/Blueprints/Triggerables/E_Directions` _array_element
      (:`NewEnumerator0`
        (set `self.EndLocation` (`KismetMathLibrary.MakeVector` _endlocation_x_5 _endlocation_y_5 (+ _endlocation_z_5 (`self.IncreaseAmount`)))))
      (:`NewEnumerator1`
        (set `self.EndLocation` (`KismetMathLibrary.MakeVector` _endlocation_x_3 _endlocation_y_3 (- _endlocation_z_3 (`self.IncreaseAmount`)))))
      (:`NewEnumerator2`
        (set `self.EndLocation` (`KismetMathLibrary.MakeVector` _endlocation_x_4 (+ _endlocation_y_4 (`self.IncreaseAmount`)) _endlocation_z_4)))
      (:`NewEnumerator3`
        (set `self.EndLocation` (`KismetMathLibrary.MakeVector` _endlocation_x_6 (- _endlocation_y_6 (`self.IncreaseAmount`)) _endlocation_z_6)))
      (:`NewEnumerator4`
        (set `self.EndLocation` (`KismetMathLibrary.MakeVector` (+ _endlocation_x (`self.IncreaseAmount`)) _endlocation_y _endlocation_z)))
      (:`NewEnumerator5`
        (set `self.EndLocation` (`KismetMathLibrary.MakeVector` (- _endlocation_x_2 (`self.IncreaseAmount`)) _endlocation_y_2 _endlocation_z_2))))))

(event `/Game/Blueprints/Triggerables/BP_Triggerable.Trigger`
  ;[1 1 1] Animates and moves the object toward the end location
  (bind (_direction _alpha) (`Timeline|MovementAlpha`)
    (:`Update`
      (`SceneComponent.K2_SetRelativeLocation` (`self.Cube`) (`KismetMathLibrary.VLerp` (`self.StartLocation`) (`self.EndLocation`) _alpha) false false))))

(fn `UserConstructionScript`
  (`parent.UserConstructionScript`)
  (`PrimitiveComponent.SetMaterial` (`self.Cube`) 0 (`self.Material`)))