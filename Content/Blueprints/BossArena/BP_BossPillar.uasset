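; BP_BossPillar is a boss arena platform that the player can trigger and the boss can target.
; On BeginPlay it finds BP_BigBoss and caches its base material.
; When the player character overlaps its collision box, it sets itself as the boss's attack platform and sends an activation message.
; AbouttobeHit briefly flashes the mesh red as a warning, and PlateformHit fires a radial force impulse as an explosion.
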(event `self.ReceiveBeginPlay`
  ;[1 1 1] Get a ref to the boss
  (bind _returnvalue (`GameplayStatics.GetActorOfClass` "/Game/Blueprints/BigBoss/BP_BigBoss.BP_BigBoss_C"))
  (set `self.BigBoss` _returnvalue)
  (set `self.BaseMaterial` (`PrimitiveComponent.GetMaterial` (`self.Cube`) 0)))

(event `self.CollistionBox.OnComponentBeginOverlap`
  (params (OverlappedComponent :type "PrimitiveComponent Object Reference") (OtherActor :type "Actor Object Reference") (OtherComp :type "PrimitiveComponent Object Reference") (OtherBodyIndex :type Integer) (bFromSweep :type Boolean) (SweepResult :type "HitResult Structure (by ref)"))
  (bind _bigboss (`self.BigBoss`))
  ;[1 1 1] On Overlap, make sure its the player, if it is, tell the boss that this is the plateform and try to activate the boss.
  (cast `/Game/ThirdPerson/Blueprints/BP_ThirdPersonCharacter` OtherActor)
  (set `/Game/Blueprints/BigBoss/BP_BigBoss.PlateformToAttack` self _bigboss)
  (message `/Game/Blueprints/BigBoss/BPI_BigBoss.ActivateBoss` _bigboss self))

(event `/Game/Blueprints/BossArena/BPI_PlateformHit.PlateformHit`
  ;[1 1 1] When plateform is hit, explode
  (`RadialForceComponent.FireImpulse` (`self.RadialForce`)))

(event `/Game/Blueprints/BossArena/BPI_PlateformHit.AboutToBeHit`
  ;[1 1 1] When a platform is about to be hit, it will flash red
  (`PrimitiveComponent.SetMaterial` (`self.Cube`) 0 "/Engine/MapTemplates/Materials/BasicAsset01.BasicAsset01")
  (`KismetSystemLibrary.Delay` 0.5)
  (`PrimitiveComponent.SetMaterial` (`self.Cube`) 0 (`self.BaseMaterial`)))

(fn `UserConstructionScript`)