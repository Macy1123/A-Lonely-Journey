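; BP_BigBoss is a test boss actor that turns to face a BP_BossPillar platform on BeginPlay, then loops through attack animations.
; AutoAttack disables mesh and sword collision, plays montages in array order despite its "random" comment, and repeats three seconds after each completes.
; The sword is hidden for the first two montages and shown for later ones.
; The construction script tints the skeletal mesh materials with BodyColor.
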(event `self.ReceiveBeginPlay`
  ;[1 1 1] Test to get the boss to know where the platform is and look at it.
  (bind _returnvalue (`GameplayStatics.GetActorOfClass` "/Game/Blueprints/BossArena/BP_BossPillar.BP_BossPillar_C"))
  (set `self.Platform` _returnvalue)
  (`self.K2_SetActorRotation` (`self.FindLookAtLocation`))
  ;[1 1 1] Loops the animations for testing
  (`self.AutoAttack`))

(event `AutoAttack`
  (bind _sword (`self.Sword`))
  (`|ExecutionSequence`
    (:`then_0`
      ;[1 1 1] Disable collisions that might hit things
      (`PrimitiveComponent.SetCollisionEnabled` (`self.SkeletalMesh`) "NoCollision")
      (`PrimitiveComponent.SetCollisionEnabled` (`self.Sword`) "NoCollision"))
    (:`then_1`
      ;[1 1 1] Selects a random animation from the list and plays it, then repeats this event
      (if (<= (`self.ArrayElementTemp`) 1)
        (`SceneComponent.SetVisibility` _sword false false)
        (else
          (`SceneComponent.SetVisibility` _sword true false)))
      (`|PlayMontage` (`self.SkeletalMesh`) (`|GetArrayItem` (`self.Animations`) (`self.ArrayElementTemp`))
        (:`OnCompleted`
          (bind _result (`/Engine/EditorBlueprintResources/StandardMacros.IncrementInt` (`self.ArrayElementTemp`))
            (:`  `
              (if (> _result (`KismetArrayLibrary.Array_LastIndex` (`self.Animations`)))
                (set `self.ArrayElementTemp` 0))
              (`KismetSystemLibrary.Delay` 3.0)
              (`self.AutoAttack`))))))))

(fn `FindLookAtLocation`
  (returns (ReturnValue :type "Rotator Structure"))
  (return (`KismetMathLibrary.FindLookAtRotation` (`self.K2_GetActorLocation`) (`self.K2_GetActorLocation` (`self.Platform`)))))

(fn `UserConstructionScript`
  (`MeshComponent.SetVectorParameterValueOnMaterials` (`self.SkeletalMesh`) "color" (`KismetMathLibrary.Conv_LinearColorToVector` (`self.BodyColor`))))